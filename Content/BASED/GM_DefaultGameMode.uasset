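; Default game mode that provides a pause toggle driven by an IsPaused flag.
; When the flag is set, PauseGame pushes WBP_PauseMenu onto P_Noa's BaseStack, stores it as CurrentMenu and unpauses the game.
; Otherwise it removes that menu and pauses, so menu visibility runs opposite to the pause state.
; PauseGame always returns false, and the event graph has no active logic.
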(fn `PauseGame`
  (returns (Success :type Boolean))
  ; PauseLogic
  (if (`self.isPaused`)
    (bind _asp_noa (cast `/Game/EpicCharacter/P_Noa` (`GameplayStatics.GetPlayerPawn` 0)))
    (bind _returnvalue (`/Game/UI/Widgets/WBP_BaseStack.PushWidgetOnStack` (`/Game/EpicCharacter/P_Noa.BaseStack` _asp_noa) "/Game/UI/Widgets/WBP_PauseMenu.WBP_PauseMenu_C"))
    (set `self.CurrentMenu` _returnvalue)
    (`GameplayStatics.SetGamePaused` false)
    (set `self.isPaused` false)
    (else
      (bind _asp_noa_2 (cast `/Game/EpicCharacter/P_Noa` (`GameplayStatics.GetPlayerPawn` 0)))
      (`/Game/UI/Widgets/WBP_BaseStack.RemoveWidgetFromStack` (`/Game/EpicCharacter/P_Noa.BaseStack` _asp_noa_2) (`self.CurrentMenu`))
      (bind _returnvalue_2 (`GameplayStatics.SetGamePaused` true))
      (set `self.isPaused` _returnvalue_2)))
  (return false))

(fn `UserConstructionScript`)