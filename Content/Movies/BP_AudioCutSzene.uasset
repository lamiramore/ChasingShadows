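; Overlap-triggered actor that silences the player's audio and starts a cutscene widget.
; When P_Noa overlaps it, a sequence first stops the character's Atmo and Music components.
; It then sets game-only input and adds a new WBP_CUTSZENE to the viewport, created with its AMIVIRGIN flag off.
; Nothing guards against repeat triggering, so each overlap creates another widget.
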(event `self.ReceiveActorBeginOverlap`
  (params (OtherActor :type "Actor Object Reference"))
  (`|ExecutionSequence`
    (:`then_0`
      (bind _asp_noa (cast `/Game/EpicCharacter/P_Noa` OtherActor))
      ; Stop Audiosources
      (`AudioComponent.Stop` (`/Game/EpicCharacter/P_Noa.Atmo` _asp_noa))
      (`AudioComponent.Stop` (`/Game/EpicCharacter/P_Noa.Music` _asp_noa)))
    (:`then_1`
      (`/Engine/EditorBlueprintResources/StandardMacros.IsValid` OtherActor
        (:`Is Valid`
          (cast `/Game/EpicCharacter/P_Noa` OtherActor)
          (`WidgetBlueprintLibrary.SetInputMode_GameOnly` (`GameplayStatics.GetPlayerController` 0))
          (bind _returnvalue (`|CreateWidget` "/Game/UI/Widgets/WBP_CUTSZENE.WBP_CUTSZENE_C" null false))
          (`UserWidget.AddToViewport` _returnvalue 0))))))

(fn `UserConstructionScript`)