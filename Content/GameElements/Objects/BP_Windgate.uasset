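; BP_Windgate is a windgate object that can start blocked by a cracked stone, which the player breaks by stomping on it.
; On BeginPlay the Blocked flag shows the stone, or hides it and destroys StoneCollision.
; When P_Noa begins overlapping StoneCollision while stomping, DestroyStone removes the CrackedStone component and Blocked is cleared, leaving StoneCollision in place.
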(event `self.ReceiveBeginPlay`
  (bind _crackedstone (`self.CrackedStone`))
  (if (`self.Blocked`)
    (`SceneComponent.SetVisibility` _crackedstone true false)
    (else
      (`SceneComponent.SetVisibility` _crackedstone false false)
      (`ActorComponent.K2_DestroyComponent` (`self.StoneCollision`)))))

(event `self.StoneCollision.OnComponentBeginOverlap`
  (params (OverlappedComponent :type "PrimitiveComponent Object Reference") (OtherActor :type "Actor Object Reference") (OtherComp :type "PrimitiveComponent Object Reference") (OtherBodyIndex :type Integer) (bFromSweep :type Boolean) (SweepResult :type "HitResult Structure (by ref)"))
  (bind _asp_noa (cast `/Game/EpicCharacter/P_Noa` OtherActor))
  (if (`/Game/EpicCharacter/P_Noa.isStomping` _asp_noa)
    (`self.DestroyStone`)
    (set `self.Blocked` false)))

(fn `DestroyStone`
  (`ActorComponent.K2_DestroyComponent` (`self.CrackedStone`)))

(fn `UserConstructionScript`)