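; BP_RandomizerComponent is an actor component that randomizes the scale and yaw of its owning actor on BeginPlay.
; It multiplies the owner's scale by a random factor between negative and positive ResizeScale, so the result can shrink toward zero or turn negative.
; It then sets a random full-circle yaw, zeroing relative pitch and roll.
; RandomizeOffset and RandomizeRotation are empty events, and Tick is unused.
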(event `self.ReceiveBeginPlay`
  (`|ExecutionSequence`
    (:`then_0`
      (`self.RandomizeSize`))
    (:`then_1`
      (`self.RandomZRotation`))))

(event `RandomizeSize`
  (bind _returnvalue (`self.GetOwner`))
  (bind _resizescale (`self.ResizeScale`))
  ; RandomizeSize
  (`Actor.SetActorScale3D` _returnvalue (* (`Actor.GetActorScale3D` _returnvalue) (`KismetMathLibrary.RandomFloatInRange` (* _resizescale -1.0) _resizescale))))

(event `RandomZRotation`
  ; Random Z Rotation
  (`Actor.K2_SetActorRelativeRotation` (`self.GetOwner`) (`KismetMathLibrary.MakeRotator` 0.0 0.0 (`KismetMathLibrary.RandomFloatInRange` 0.0 360.0)) false false))

(event `RandomizeOffset`)

(event `RandomizeRotation`)