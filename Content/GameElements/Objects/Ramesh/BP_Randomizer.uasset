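; BP_Randomizer is an actor whose point light changes to a random color and intensity about every half second.
; Tick drives RandomizeLight through a Delay, picking from a fixed color palette and an intensity between min and max variables.
; ModifyMesh on BeginPlay and MoveMesh on Tick use zero vectors, so the mesh never moves or rotates and is scaled to zero.
; A SetStaticMesh node is left unconnected.
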(event `self.ReceiveBeginPlay`
  (`self.ModifyMesh`))

(event `self.ReceiveTick`
  (params (DeltaSeconds :type "Float (single-precision)"))
  (`self.MoveMesh` DeltaSeconds)
  (`KismetSystemLibrary.Delay` 0.5)
  (`self.RandomizeLight`))

(fn `ModifyMesh`
  (bind _mymesh (`self.MyMesh`))
  (`SceneComponent.K2_AddWorldOffset` _mymesh (0.0 0.0 0.0) false false)
  (`SceneComponent.K2_AddWorldRotation` :`self` _mymesh)
  (`SceneComponent.SetWorldScale3D` _mymesh (0.0 0.0 0.0)))

(fn `MoveMesh`
  (params (B :type "Float (single-precision)"))
  (`SceneComponent.K2_AddWorldOffset` (`self.MyMesh`) (* (0.0 0.0 0.0) B) false false))

(fn `RandomizeLight`
  (bind _pointlight (`self.PointLight`))
  (`LightComponent.SetLightColor` _pointlight (`KismetArrayLibrary.Array_Random` (`|MakeArray` (struct :`G` 0.974891 :`B` 1.0 :`A` 1.0) (struct :`R` 0.004806 :`G` 1.0 :`B` 0.023375 :`A` 1.0) (struct :`R` 1.0 :`G` 0.01319 :`A` 1.0) (struct :`R` 1.0 :`G` 0.269505 :`A` 1.0) (struct :`R` 0.854329 :`G` 1.0 :`B` 0.054648 :`A` 1.0) (struct :`R` 0.320973 :`G` 0.154786 :`B` 0.552083 :`A` 1.0) (struct :`R` 0.828125 :`G` 0.145849 :`B` 0.721683 :`A` 1.0) :!type "LinearColor Structure")) true)
  (`LightComponent.SetIntensity` _pointlight (`KismetMathLibrary.RandomFloatInRange` (`self.LightIntensity_Min`) (`self.LightIntensity_Max`))))

(fn `UserConstructionScript`)