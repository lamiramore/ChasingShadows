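; BP_Gravestone is a gravestone prop actor that randomizes its own placement and size so copies look varied.
; On BeginPlay it shifts the Cube component vertically within a height limit, then replaces actor rotation with random yaw and slight roll and pitch tilt.
; It multiplies actor scale uniformly by a random factor between zero and ResizeBy, despite a comment describing 20% variation either way.
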(event `self.ReceiveBeginPlay`
  (bind _resizeby (`self.ResizeBy`))
  (bind _maxheightdifference (`self.MaxHeightDifference`))
  (bind _maxrotationxy (`self.MaxRotationXY`))
  (bind _returnvalue (`KismetMathLibrary.RandomFloatInRange` (* _maxrotationxy -1.0) _maxrotationxy))
  ; Zufälliger Offset (Z-Achse)
  (`SceneComponent.K2_AddWorldOffset` (`self.Cube`) (`KismetMathLibrary.MakeVector` 0.0 0.0 (`KismetMathLibrary.RandomFloatInRange` (* _maxheightdifference -1.0) _maxheightdifference)) false false)
  ; Zufällige Rotation (Z-Achse) + Neigung (X- + Y-Achse)
  (`self.K2_SetActorRotation` (`KismetMathLibrary.MakeRotator` _returnvalue _returnvalue (`KismetMathLibrary.RandomFloatInRange` (* 0.0 -1.0) (`self.MaxRotationZ`))))
  ; Zufällige Größe (20% grösser oder kleiner)
  (`self.SetActorScale3D` (* (`self.GetActorScale3D`) (`KismetMathLibrary.RandomFloatInRange` (* _resizeby 0.0) _resizeby))))

(fn `UserConstructionScript`)