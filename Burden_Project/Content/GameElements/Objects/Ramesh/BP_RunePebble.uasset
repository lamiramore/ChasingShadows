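; BP_RunePebble is a rune stone prop that glows brighter as the player approaches.
; BeginPlay creates a dynamic material instance on the mesh.
; Tick scales its EmissiveStrength inversely and linearly with the player pawn's distance, fading to zero at MaxGlowDist.
; A separate ApplyRandomRot event gives the mesh a random rotation on all axes, but nothing in this Blueprint calls it.
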(event `ApplyRandomRot`
  (bind _returnvalue (`KismetMathLibrary.RandomFloatInRange` 0.0 360.0))
  ; Apply Random Rotation Event
  (`SceneComponent.K2_SetRelativeRotation` (`self.Mesh`) (`KismetMathLibrary.MakeRotator` _returnvalue _returnvalue _returnvalue) false false))

(event `self.ReceiveBeginPlay`
  ; Spawn Stones
  (bind _returnvalue (`PrimitiveComponent.CreateDynamicMaterialInstance` (`self.Mesh`) 0 null "None"))
  (set `self.MID` _returnvalue))

(event `self.ReceiveTick`
  (params (DeltaSeconds :type "Float (single-precision)"))
  ; Set Emission every Tick
  (`MaterialInstanceDynamic.SetScalarParameterValue` (`self.MID`) "EmissiveStrength" (* (- 1.0 (`KismetMathLibrary.FClamp` (/ (`KismetMathLibrary.VSize` (- (`self.K2_GetActorLocation` (`GameplayStatics.GetPlayerPawn` 0)) (`self.K2_GetActorLocation`))) (`self.MaxGlowDist`)))) 3.0)))

(fn `UserConstructionScript`)