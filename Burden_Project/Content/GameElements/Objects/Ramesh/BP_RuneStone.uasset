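; BP_RuneStone is a rune stone object whose emissive glow turns on the first time the P_Noa character enters its sphere trigger.
; BeginPlay creates a dynamic material instance on the mesh.
; A DoOnce-gated overlap plays a timeline that drives the EmissiveStrength parameter, scaled by a maximum strength, then sets RunesOn when finished.
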(event `self.ReceiveBeginPlay`
  (bind _returnvalue (`PrimitiveComponent.CreateDynamicMaterialInstance` (`self.Mesh`) 0 null "None"))
  (set `self.MID` _returnvalue))

(event `self.Sphere.OnComponentBeginOverlap`
  (params (OverlappedComponent :type "PrimitiveComponent Object Reference") (OtherActor :type "Actor Object Reference") (OtherComp :type "PrimitiveComponent Object Reference") (OtherBodyIndex :type Integer) (bFromSweep :type Boolean) (SweepResult :type "HitResult Structure (by ref)"))
  (cast `/Game/EpicCharacter/P_Noa` OtherActor)
  (`/Engine/EditorBlueprintResources/StandardMacros.DoOnce` false
    (:`Completed`
      (bind (_direction _emission) (`Timeline|TL_Emission`)
        (:`Update`
          (`MaterialInstanceDynamic.SetScalarParameterValue` (`self.MID`) "EmissiveStrength" (* _emission (`self.MaxEmissiveStrength`))))
        (:`Finished`
          (set `self.RunesOn` true))))))

(fn `UserConstructionScript`)